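; Lobby player controller for the EGSDK backend, handling login, registration, password changes, email codes, key-value account updates and mail.
; Each API event sends a VaRest GET request and reports through tip widgets, with a looping timer and Tick check flagging timeouts.
; Successful login caches account data in GI_EGSDK, opens the UI_EGSDK_Power widget and fetches mail into the game instance.
; Helpers show the login UI, build mail list entries and convert scores to rank tiers.
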(event `self.ReceiveTick`
  (params (DeltaSeconds :type "Float (single-precision)"))
  (if (> (`self.time`) 7.0)
    (bind _returnvalue (`|CreateWidget` "/EGSDK/UI/Tip/UI_EGSDK_Tip.UI_EGSDK_Tip_C" (`GameplayStatics.GetPlayerController` 0) "连接后端服务器超时!#Time_out"))
    (`UserWidget.AddToViewport` _returnvalue 8)
    (`KismetSystemLibrary.K2_ClearAndInvalidateTimerHandle` (`self.NewVar_0`))
    (set `self.time` 0.0)))

(event `timeout`
  (set `self.time` (+ (`self.time`) 1.0)))

(event `LoginAPI`
  (params (Account :type String) (password :type String) (UI :type "Widget Object Reference"))
  (set `self.time` 0.0)
  (bind _returnvalue (`KismetSystemLibrary.K2_SetTimerDelegate` (delegate `timeout`) 1.0 true))
  (set `self.NewVar_0` _returnvalue)
  (bind _returnvalue_2 (`VaRestSubsystem.ConstructVaRestRequestExt` (subsystem `VaRestSubsystem`) "GET" "x_www_form_urlencoded_url"))
  (bind _returnvalue_3 (`VaRestRequestJSON.GetRequestObject` _returnvalue_2))
  (`VaRestJsonObject.SetStringField` _returnvalue_3 "u" Account)
  (`VaRestJsonObject.SetStringField` _returnvalue_3 "p" password)
  (bind _result (`VaRestRequestJSON.ApplyURL` _returnvalue_2 (`KismetStringLibrary.Concat_StrStr` (`self.IP`) "/login")))
  (`KismetSystemLibrary.K2_ClearAndInvalidateTimerHandle` (`self.NewVar_0`))
  (bind _returnvalue_4 (`VaRestJsonValue.AsString` (`VaRestJsonObject.GetField` _result "success")))
  (if (`KismetStringLibrary.EqualEqual_StrStr` _returnvalue_4 "Pass")
    (`|ExecutionSequence`
      (:`then_0`
        (`KismetSystemLibrary.PrintString` _returnvalue_4)
        (bind _returnvalue_5 (`VaRestJsonValue.AsString` (`VaRestJsonObject.GetField` _result "id")))
        (bind _output_get (set `self.Account` _returnvalue_5)))
      (:`then_1`
        (bind _returnvalue_6 (`VaRestJsonValue.AsString` (`VaRestJsonObject.GetField` _result "username")))
        (bind _output_get_2 (set `self.Username` _returnvalue_6)))
      (:`then_2`
        (bind _output_get_3 (set `self.bp` (`VaRestJsonValue.AsString` (`VaRestJsonObject.GetField` _result "userbp"))))
        (bind _asgi_egsdk (cast `/EGSDK/Lobby/GI_EGSDK` (`GameplayStatics.GetGameInstance`)))
        (bind _output_get_4 (set `/EGSDK/Lobby/GI_EGSDK.Account` _returnvalue_5 _asgi_egsdk))
        (set `/EGSDK/Lobby/GI_EGSDK.Username` _returnvalue_6 _asgi_egsdk)
        (set `/EGSDK/Lobby/GI_EGSDK.bp` (`KismetStringLibrary.Conv_StringToInt` _output_get_3) _asgi_egsdk)
        (set `/EGSDK/Lobby/GI_EGSDK.rp` (`KismetStringLibrary.Conv_StringToInt` (`VaRestJsonValue.AsString` (`VaRestJsonObject.GetField` _result "rp"))) _asgi_egsdk)
        (`KismetSystemLibrary.Delay` 1.0)
        (bind _returnvalue_7 (`|CreateWidget` "/EGSDK/UI/Tip/UI_EGSDK_Power.UI_EGSDK_Power_C" self (`KismetTextLibrary.Conv_StringToText` _output_get_2) (`KismetTextLibrary.Conv_StringToText` _output_get) (`self.大厅`)))
        (`UserWidget.AddToViewport` _returnvalue_7 3)
        (`Widget.RemoveFromParent` UI)
        (`self.GetMail` _output_get_4)))
    (else
      (bind _returnvalue_8 (`|CreateWidget` "/EGSDK/UI/Tip/UI_EGSDK_Tip.UI_EGSDK_Tip_C" self (`KismetTextLibrary.Conv_StringToText` _returnvalue_4)))
      (`UserWidget.AddToViewport` _returnvalue_8 0))))

(event `ChangePassword`
  (params (account :type String) (mail :type String) (password :type String) (`邮箱验证码` :type String))
  (set `self.time` 0.0)
  (bind _returnvalue (`KismetSystemLibrary.K2_SetTimerDelegate` (delegate `timeout`) 1.0 true))
  (set `self.NewVar_0` _returnvalue)
  (bind _returnvalue_2 (`VaRestSubsystem.ConstructVaRestRequestExt` (subsystem `VaRestSubsystem`) "GET" "x_www_form_urlencoded_url"))
  (bind _returnvalue_3 (`VaRestRequestJSON.GetRequestObject` _returnvalue_2))
  (`VaRestJsonObject.SetStringField` _returnvalue_3 "account" account)
  (`VaRestJsonObject.SetStringField` _returnvalue_3 "mail" mail)
  (`VaRestJsonObject.SetStringField` _returnvalue_3 "password" password)
  (`VaRestJsonObject.SetStringField` _returnvalue_3 "mp" `邮箱验证码`)
  (bind _result (`VaRestRequestJSON.ApplyURL` _returnvalue_2 (`KismetStringLibrary.Concat_StrStr` (`self.IP`) "/changepassword")))
  (`KismetSystemLibrary.K2_ClearAndInvalidateTimerHandle` (`self.NewVar_0`))
  (bind _returnvalue_4 (`VaRestJsonValue.AsString` (`VaRestJsonObject.GetField` _result "success")))
  (if (`KismetStringLibrary.EqualEqual_StrStr` _returnvalue_4 "Pass")
    (bind _returnvalue_5 (`|CreateWidget` "/EGSDK/UI/Tip/UI_EGSDK_Tip.UI_EGSDK_Tip_C" null "修改成功请重新登录！"))
    (`UserWidget.AddToViewport` _returnvalue_5 0)
    (else
      (bind _returnvalue_6 (`|CreateWidget` "/EGSDK/UI/Tip/UI_EGSDK_Tip.UI_EGSDK_Tip_C" null (`KismetTextLibrary.Conv_StringToText` _returnvalue_4)))
      (`UserWidget.AddToViewport` _returnvalue_6 0))))

(event `Change`
  (params (Value :type String) (Key :type String) (Account :type String))
  (set `self.time` 0.0)
  (bind _returnvalue (`KismetSystemLibrary.K2_SetTimerDelegate` (delegate `timeout`) 1.0 true))
  (set `self.NewVar_0` _returnvalue)
  (bind _returnvalue_2 (`VaRestSubsystem.ConstructVaRestRequestExt` (subsystem `VaRestSubsystem`) "GET" "x_www_form_urlencoded_url"))
  (bind _returnvalue_3 (`VaRestRequestJSON.GetRequestObject` _returnvalue_2))
  (`VaRestJsonObject.SetStringField` _returnvalue_3 "account" Account)
  (`VaRestJsonObject.SetStringField` _returnvalue_3 "key" Key)
  (`VaRestJsonObject.SetStringField` _returnvalue_3 "value" Value)
  (bind _result (`VaRestRequestJSON.ApplyURL` _returnvalue_2 (`KismetStringLibrary.Concat_StrStr` (`self.IP`) "/change")))
  (`KismetSystemLibrary.K2_ClearAndInvalidateTimerHandle` (`self.NewVar_0`))
  (if (not (`KismetStringLibrary.EqualEqual_StrStr` (`VaRestJsonValue.AsString` (`VaRestJsonObject.GetField` _result "success")) "Pass"))
    (bind _returnvalue_4 (`|CreateWidget` "/EGSDK/UI/Tip/UI_EGSDK_Tip.UI_EGSDK_Tip_C" null "网络异常，请检查网络是否通畅"))
    (`UserWidget.AddToViewport` _returnvalue_4 10)))

(event `RegistarAPI`
  (params (`用户名` :type String) (`密码` :type String) (`邮箱` :type String) (`验证码` :type String))
  (set `self.time` 0.0)
  (bind _returnvalue (`KismetSystemLibrary.K2_SetTimerDelegate` (delegate `timeout`) 1.0 true))
  (set `self.NewVar_0` _returnvalue)
  (bind _returnvalue_2 (`VaRestSubsystem.ConstructVaRestRequestExt` (subsystem `VaRestSubsystem`) "GET" "x_www_form_urlencoded_url"))
  (bind _returnvalue_3 (`VaRestRequestJSON.GetRequestObject` _returnvalue_2))
  (`VaRestJsonObject.SetStringField` _returnvalue_3 "n" `用户名`)
  (`VaRestJsonObject.SetStringField` _returnvalue_3 "p" `密码`)
  (`VaRestJsonObject.SetStringField` _returnvalue_3 "mail" `邮箱`)
  (`VaRestJsonObject.SetStringField` _returnvalue_3 "mp" `验证码`)
  (bind _result (`VaRestRequestJSON.ApplyURL` _returnvalue_2 (`KismetStringLibrary.Concat_StrStr` (`self.IP`) "/reg")))
  (`KismetSystemLibrary.K2_ClearAndInvalidateTimerHandle` (`self.NewVar_0`))
  (bind _returnvalue_4 (`VaRestJsonValue.AsString` (`VaRestJsonObject.GetField` _result "success")))
  (if (`KismetStringLibrary.EqualEqual_StrStr` _returnvalue_4 "Pass")
    (bind _returnvalue_5 (`|CreateWidget` "/EGSDK/UI/Tip/UI_EGSDK_Tip.UI_EGSDK_Tip_C" null (`|FormatText` "请记住您的账号：{a}" (`VaRestJsonValue.AsString` (`VaRestJsonObject.GetField` _result "account")))))
    (`UserWidget.AddToViewport` _returnvalue_5 10)
    (else
      (bind _returnvalue_6 (`|CreateWidget` "/EGSDK/UI/Tip/UI_EGSDK_Tip.UI_EGSDK_Tip_C" null (`KismetTextLibrary.Conv_StringToText` _returnvalue_4)))
      (`UserWidget.AddToViewport` _returnvalue_6 10))))

(event `发送验证码`
  (params (`邮箱地址` :type String))
  (bind _returnvalue (`KismetSystemLibrary.K2_SetTimerDelegate` (delegate `timeout`) 1.0 true))
  (set `self.NewVar_0` _returnvalue)
  (bind _returnvalue_2 (`VaRestSubsystem.ConstructVaRestRequestExt` (subsystem `VaRestSubsystem`) "GET" "x_www_form_urlencoded_url"))
  (`VaRestJsonObject.SetStringField` (`VaRestRequestJSON.GetRequestObject` _returnvalue_2) "email" `邮箱地址`)
  (bind _result (`VaRestRequestJSON.ApplyURL` _returnvalue_2 (`KismetStringLibrary.Concat_StrStr` (`self.IP`) "/requestmailpw")))
  (`KismetSystemLibrary.K2_ClearAndInvalidateTimerHandle` (`self.NewVar_0`))
  (bind _returnvalue_3 (`|CreateWidget` "/EGSDK/UI/Tip/UI_EGSDK_Tip.UI_EGSDK_Tip_C" null (`KismetTextLibrary.Conv_StringToText` (`VaRestJsonValue.AsString` (`VaRestJsonObject.GetField` _result "success")))))
  (`UserWidget.AddToViewport` _returnvalue_3 10))

(event `GetMail`
  (params (Account :type String))
  (bind _asgi_egsdk (cast `/EGSDK/Lobby/GI_EGSDK` (`GameplayStatics.GetGameInstance`) :!pure true))
  (bind _mail_title (`/EGSDK/Lobby/GI_EGSDK.mail_Title` _asgi_egsdk))
  (bind _mail_content (`/EGSDK/Lobby/GI_EGSDK.mail_Content` _asgi_egsdk))
  (bind _mail_state (`/EGSDK/Lobby/GI_EGSDK.mail_State` _asgi_egsdk))
  (bind _mail_id (`/EGSDK/Lobby/GI_EGSDK.mail_ID` _asgi_egsdk))
  (set `self.time` 0.0)
  (bind _returnvalue (`KismetSystemLibrary.K2_SetTimerDelegate` (delegate `timeout`) 1.0 true))
  (set `self.NewVar_0` _returnvalue)
  (bind _returnvalue_2 (`VaRestSubsystem.ConstructVaRestRequestExt` (subsystem `VaRestSubsystem`) "GET" "x_www_form_urlencoded_url"))
  (`VaRestJsonObject.SetStringField` (`VaRestRequestJSON.GetRequestObject` _returnvalue_2) "account" Account)
  (bind _result (`VaRestRequestJSON.ApplyURL` _returnvalue_2 (`KismetStringLibrary.Concat_StrStr` (`self.IP_邮箱系统`) "/get")))
  (`KismetSystemLibrary.K2_ClearAndInvalidateTimerHandle` (`self.NewVar_0`))
  (bind _returnvalue_3 (`VaRestJsonValue.AsString` (`VaRestJsonObject.GetField` _result "success")))
  (if (`KismetStringLibrary.EqualEqual_StrStr` _returnvalue_3 "Pass")
    (`KismetArrayLibrary.Array_Clear` _mail_id)
    (`KismetArrayLibrary.Array_Clear` _mail_title)
    (`KismetArrayLibrary.Array_Clear` _mail_content)
    (`KismetArrayLibrary.Array_Clear` _mail_state)
    (for _array_element (`VaRestJsonValue.AsArray` (`VaRestJsonObject.GetField` _result "id"))
      (`KismetArrayLibrary.Array_Add` _mail_id (`VaRestJsonValue.AsString` _array_element)))
    (for _array_element_2 (`VaRestJsonValue.AsArray` (`VaRestJsonObject.GetField` _result "title"))
      (`KismetArrayLibrary.Array_Add` _mail_title (`VaRestJsonValue.AsString` _array_element_2)))
    (for _array_element_3 (`VaRestJsonValue.AsArray` (`VaRestJsonObject.GetField` _result "content"))
      (`KismetArrayLibrary.Array_Add` _mail_content (`VaRestJsonValue.AsString` _array_element_3)))
    (for _array_element_4 (`VaRestJsonValue.AsArray` (`VaRestJsonObject.GetField` _result "state"))
      (`KismetArrayLibrary.Array_Add` _mail_state (`VaRestJsonValue.AsString` _array_element_4)))
    (else
      (bind _returnvalue_4 (`|CreateWidget` "/EGSDK/UI/Tip/UI_EGSDK_Tip.UI_EGSDK_Tip_C" self (`KismetTextLibrary.Conv_StringToText` _returnvalue_3)))
      (`UserWidget.AddToViewport` _returnvalue_4 0))))

(event `Showmail`
  (params (Mail_ID :type "Array of String") (Mail_Title :type "Array of String") (Mail_Content :type "Array of String") (Mail_State :type "Array of String") (TargetUI :type "/EGSDK/UI/MailSystem/UI_EGSDK_ShowMail Object Reference"))
  (for _index (range (`KismetArrayLibrary.Array_Length` Mail_ID))
    (bind _returnvalue (`|CreateWidget` "/EGSDK/UI/MailSystem/UI_EGSDK_MailBody.UI_EGSDK_MailBody_C" self (`|GetArrayItem` Mail_ID _index) (`|GetArrayItem` Mail_Title _index) (`KismetTextLibrary.Conv_StringToText` (`|GetArrayItem` Mail_Content _index)) (`|GetArrayItem` Mail_State _index)))
    (`PanelWidget.AddChild` (`/EGSDK/UI/MailSystem/UI_EGSDK_ShowMail.Body` TargetUI) _returnvalue)))

(fn `UserConstructionScript`)

(fn `显示外部登录UI(EG)`
  (params (PlayerController :type "PlayerController Object Reference"))
  (returns (ReturnUI :type "Widget Object Reference"))
  (bind _returnvalue (`|CreateWidget` "/EGSDK/UI/UI_EGSDK_Login.UI_EGSDK_Login_C" PlayerController))
  (`UserWidget.AddToViewport` _returnvalue 0)
  (return _returnvalue))

(fn `段位判断`
  (params (`段位分数` :type Integer))
  (returns (`段位序号` :type Integer) (`段位名` :type String) (`下一段位分数` :type Integer))
  (bind _returnvalue (/ `段位分数` 100))
  (bind _returnvalue_2 (/ (- `段位分数` 1000) 100))
  (bind _output_get (set `self.段位序号` _returnvalue_2))
  (`KismetSystemLibrary.PrintText` (`KismetTextLibrary.Conv_IntToText` _output_get))
  (return _returnvalue_2 (`BlueprintMapLibrary.Map_Find` (`self.段位分段`) (* _returnvalue 100)) (* (+ _returnvalue 1) 100)))